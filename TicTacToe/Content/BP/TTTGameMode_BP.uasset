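; Game mode for a tic-tac-toe game that tracks whose turn it is and detects a draw.
; On BeginPlay it makes X the first player and binds a handler to the PlayerFinished event.
; Each finished turn increments a counter, then either flips the current player or prints a draw once all nine moves are used.
; No win check takes place here.
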(event `self.ReceiveBeginPlay`
  (set `self.PlayerIsX` true)
  (add `self.PlayerFinished` (delegate `PlayerFinished_Event`)))

(event `PlayerFinished_Event`
  (bind _result (`/Engine/EditorBlueprintResources/StandardMacros.IncrementInt` (`self.TurnCounter`))
    (:`  `
      (set `self.TurnCounter` _result)
      (if (>= (`self.TurnCounter`) 9)
        (`KismetSystemLibrary.PrintString` "Draw")
        (else
          (set `self.PlayerIsX` (not (`self.PlayerIsX`))))))))

(fn `UserConstructionScript`)