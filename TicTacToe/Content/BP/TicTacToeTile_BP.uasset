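; Clickable tic-tac-toe board tile that claims itself for the current player when clicked while empty.
; It reads whose turn it is from TTTGameMode_BP, records its state, shows the X or O mesh and swaps the plane to the blue or orange material.
; It then asks its owning grid for a victory check and tells the game mode either that a player won or that the turn is finished.
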(event `self.Plane.OnClicked`
  (params (TouchedComponent :type "PrimitiveComponent Object Reference") (ButtonPressed :type "Key Structure"))
  (if (== (`self.TileState`) 0)
    (bind _astttgame_mode_bp (cast `/Game/BP/TTTGameMode_BP` (`GameplayStatics.GetGameMode`)))
    (bind _playerisx (`/Game/BP/TTTGameMode_BP.PlayerIsX` _astttgame_mode_bp))
    (if _playerisx
      (set `self.TileState` 1)
      (`SceneComponent.SetVisibility` (`self.X`) true true)
      (`PrimitiveComponent.SetMaterial` (`self.Plane`) 0 "/Game/Puzzle/Meshes/BlueMaterial.BlueMaterial")
      (else
        (set `self.TileState` 2)
        (`SceneComponent.SetVisibility` (`self.O`) true true)
        (`PrimitiveComponent.SetMaterial` (`self.Plane`) 0 "/Game/Puzzle/Meshes/OrangeMaterial.OrangeMaterial")))
    (bind _returnvalue (`TicTacToeTileGrid.VictoryCheck` (`self.OwningGrid`) (`self.TileNum`) _playerisx))
    (if (!= _returnvalue 0)
      (`/Game/BP/TTTGameMode_BP.PlayerWon` _astttgame_mode_bp _returnvalue)
      (else
        (`/Game/BP/TTTGameMode_BP.PlayerFinished` _astttgame_mode_bp)))))

(fn `UserConstructionScript`)